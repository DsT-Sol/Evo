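; Touch and mouse orbit camera that circles a pivot with pinch zoom, clamped tracking and optional pitch/yaw limits.
; BeginPlay spawns BP_TouchManager; Tick turns input into smoothed offsets and rotations with optional drift, or eases toward a transition yaw.
; Polling timers set drift direction and trigger sleep, attract and easing states after inactivity.
; It also follows reported locations outside a radius, fades via a material sphere and shows debug limit arcs.
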(event Custom|DriftChoice
  (bind _mouse_x (Variables|Default|GetMouse%20X))
  (bind _touch_x (Variables|Default|GetTouch%20X))
  (bind _returnvalue (+ _mouse_x _touch_x))
  ;[1 1 1] Loop to update drift velocities
  (if (> _returnvalue 0.005)
    (Variables|Default|SetDrift%20Amount 0.02)
    (elif (< _returnvalue -0.005)
      (Variables|Default|SetDrift%20Amount -0.02))))

(event Custom|Asleep
  ;[1 1 1] Attract Timers
  (Default|CallGonetoSleep)
  (Utilities|FlowControl|DoOnce true) ; enters at Reset
)

(event Custom|FadeToReset
  ;[1 1 1] Fade on Restart
  (Rendering|SetVisibility (Variables|Default|GetFadeSphere) true false)
  (bind _fadetrack (Timeline|FadeTimer PlayFromStart)
    (:Update
      (Rendering|Material|SetScalarParameterValue (Variables|Default|GetFadeMat) "Fade" _fadetrack :!class /Script/Engine.MaterialInstanceDynamic))
    (:Finished
      (Default|CallDoneFade))))

(event Custom|EaseTimer
  ;[1 1 1] Attract Timers
  (Variables|Default|SetPinchEase true))

(event Custom|Alone
  ;[1 1 1] Attract Timers
  (Variables|Default|SetAttractMode true))

(event Custom|FadeUp
  ;[1 1 1] Fade Recovery
  (Rendering|Material|SetScalarParameterValue (Variables|Default|GetFadeMat) "Fade" 1.0 :!class /Script/Engine.MaterialInstanceDynamic)
  (Rendering|SetVisibility (Variables|Default|GetFadeSphere) true false)
  (bind _newtrack_0 (Timeline|FadeUpTrack Play)
    (:Update
      (Rendering|Material|SetScalarParameterValue (Variables|Default|GetFadeMat) "Fade" _newtrack_0 :!class /Script/Engine.MaterialInstanceDynamic))
    (:Finished
      (Rendering|SetVisibility (Variables|Default|GetFadeSphere) false false))))

(event Custom|PinchCheck
  ;[1 1 1] Attract Timers
  (if (or (Variables|Default|GetPinch) (Variables|Default|GetOverallTouch))
    (Utilities|FlowControl|Sequence
      (:then_0
        (goto _label Reset))
      (:then_1
        (Variables|Default|SetPinchEase false)
        (Variables|Default|SetAttractMode false)
        (Utilities|Time|ClearTimerbyFunctionName 0 "Asleep")
        (Utilities|Time|ClearTimerbyFunctionName 0 "Alone")
        (Utilities|Time|ClearTimerbyFunctionName 0 "EaseTimer")))
    (else
      (Utilities|FlowControl|DoOnce true :!label _label
        (:Completed
          (Utilities|Time|SetTimerbyFunctionName 0 "Asleep" (Variables|Default|GetIdle%20Timer))
          (Utilities|Time|SetTimerbyFunctionName 0 "Alone" (Variables|Default|GetAttract%20Timer))
          (Utilities|Time|SetTimerbyFunctionName 0 "EaseTimer" 16.0))))))

(event Custom|ForceTransition
  ;[1 1 1] Attract Timers
  (Utilities|Time|ClearTimerbyFunctionName 0 "Asleep")
  (Utilities|Time|ClearTimerbyFunctionName 0 "Alone")
  (Utilities|Time|ClearTimerbyFunctionName 0 "EaseTimer"))

(event EventBeginPlay
  (bind _orbitarcindicator (Variables|Default|GetOrbitArcIndicator))
  (bind _returnvalue (Transformation|GetWorldScale _orbitarcindicator))
  ;[1 1 1] Initialize
  (bind _returnvalue_2 (Game|SpawnActorfromClass "/Game/Cameras/BP_TouchManager.BP_TouchManager_C" (Transformation|GetActorTransform) "AlwaysSpawn" self 0))
  (Variables|Default|SetLocalTouchManager _returnvalue_2)
  ;[1 1 1] Loop to update drift velocities
  (Utilities|Time|SetTimerbyFunctionName 0 "Alone" (Variables|Default|GetAttract%20Timer))
  (Utilities|Time|SetTimerbyEvent (delegate Custom|DriftChoice) 0.05 true)
  (Utilities|Time|SetTimerbyFunctionName 0 "PinchCheck" 0.05 true)
  ;[1 1 1] Initial Yaw
  (Variables|Default|SetInitialYaw (.Yaw (Math|Rotator|BreakRotator (Transformation|GetWorldRotation (Variables|Default|GetOrbitPoint)))))
  ;[1 1 1] Arc Debug
  (Development|SetHiddeninGame _orbitarcindicator (not (Variables|CameraAngles|GetbDebugArcs)) false)
  (Transformation|SetWorldScale3D _orbitarcindicator (Math|Vector|SelectVector (* _returnvalue 0.75) _returnvalue (Variables|CameraAngles|GetbDebugArcs))))

(event EventEvoLocation
  (params (Location :type Vector :default "0, 0, 0"))
  (bind _cameratrackingradius (Variables|CameraSettings|GetCameraTrackingRadius))
  ;[1 1 1] Actor Tracking After Leaving Specific Area
  (bind _output_get (Variables|Default|SetCurrentEvoLocation Location))
  (if (or (> (.X (Math|Vector|BreakVector _output_get)) _cameratrackingradius) (> (.Y (Math|Vector|BreakVector _output_get)) _cameratrackingradius))
    (Transformation|SetActorLocation (Math|Vector|Lerp(Vector) _output_get (Transformation|GetActorLocation) (+ (/ (Variables|CameraSettings|GetCameraTrackSpeed) 1e+02) 0.9)) false false)))

(event EventTick
  (params (DeltaSeconds :type Float%20%28single-precision%29))
  ;[1 1 1] Interaction controls
  (Variables|Default|SetTickTime DeltaSeconds)
  (if (Variables|Default|GetbFindTarget)
    (Utilities|FlowControl|Sequence
      (:then_0
        (|TransitionBehavior))
      (:then_1
        (|ShiftDistanceofCamera :!label _label)))
    (else
      (Utilities|FlowControl|Sequence
        (:then_0
          (goto _label))
        (:then_1
          (|ApplyPinch)
          (if (Variables|Default|GetbAllowOrbit)
            (|SetCameraPitch)
            (|SetCameraYaw)
            (|ApplyDriftInertia)))
        (:then_2
          (|DetermineCameraDistance))))))

(fn ConstructionScript
  (bind _pitcharcindicator (Variables|Default|GetPitchArcIndicator))
  (bind _blimitorbit (Variables|CameraAngles|GetbLimitOrbit))
  ;[1 1 1] Preplace camera
  (Transformation|SetRelativeLocation (Variables|Default|GetCineCamera) (Math|Vector|MakeVector (- 0.0 (Variables|CameraSettings|GetOrbit%20Distance)) 0.0 0.0) false false)
  ;[1 1 1] Fade Setup
  (bind _returnvalue (Rendering|Material|CreateDynamicMaterialInstance (Variables|Default|GetFadeSphere) 0 "/Game/Cameras/Effects/Materials/M_CameraFade.M_CameraFade" "None" :!class /Script/Engine.PrimitiveComponent))
  (Variables|Default|SetFadeMat _returnvalue)
  ;[1 1 1] Setup Debug Arcs and Limits
  (Utilities|FlowControl|Sequence
    (:then_0
      (bind _returnvalue_2 (Rendering|Material|CreateDynamicMaterialInstance (Variables|Default|GetOrbitArcIndicator) 0 0 "None" :!class /Script/Engine.PrimitiveComponent))
      (bind _output_get (Variables|Default|SetOrbitRingMat _returnvalue_2))
      (Rendering|Material|SetScalarParameterValue _output_get "MinPercent" (Math|Float|SelectFloat (/ (Variables|CameraAngles|GetMin%20Orbit%20Arc) 1.8e+02) 1.0 _blimitorbit) :!class /Script/Engine.MaterialInstanceDynamic)
      (Rendering|Material|SetScalarParameterValue _output_get "MaxPercent" (Math|Float|SelectFloat (/ (Variables|CameraAngles|GetMax%20Orbit%20Arc) 1.8e+02) 1.0 _blimitorbit) :!class /Script/Engine.MaterialInstanceDynamic)
      (Transformation|SetWorldScale3D (Variables|Default|GetOrbitArcIndicator) (Math|Conversions|ToVector(Float) (/ (Variables|CameraSettings|GetOrbit%20Distance) 1e+02)))
      (Transformation|SetRelativeRotation (Variables|Default|GetPitchPoint) (Math|Rotator|MakeRotator 0.0 (- 0.0 (Variables|CameraAngles|GetInitial%20Pitch)) 0.0) false false))
    (:then_1
      (bind _returnvalue_3 (Rendering|Material|CreateDynamicMaterialInstance _pitcharcindicator 0 0 "None" :!class /Script/Engine.PrimitiveComponent))
      (bind _output_get_2 (Variables|Default|SetPitchRingMat _returnvalue_3))
      (Transformation|SetWorldScale3D _pitcharcindicator (Math|Conversions|ToVector(Float) (/ (Variables|CameraSettings|GetOrbit%20Distance) 1e+02)))
      (Rendering|Material|SetScalarParameterValue _output_get_2 "MinPercent" (/ (Variables|CameraAngles|GetMin%20Pitch) 1.8e+02) :!class /Script/Engine.MaterialInstanceDynamic)
      (Rendering|Material|SetScalarParameterValue _output_get_2 "MaxPercent" (/ (Variables|CameraAngles|GetMax%20Pitch) 1.8e+02) :!class /Script/Engine.MaterialInstanceDynamic)
      (Components|Activation|SetAutoActivate (Variables|Default|GetMotionController) (Variables|InputResponse|GetbUseMotionControllerTracking)))))

(fn FadeComplete)

(fn LocalTruncate
  (params (Incoming :type Float%20%28double-precision%29))
  (return (* (Math|Float|Truncate (* 1000 Incoming)) 0.001)))

(fn SetOrbitDistance
  (params (NewOrbitDistance :type Float%20%28double-precision%29))
  (Variables|CameraSettings|SetOrbit%20Distance NewOrbitDistance)
  (Transformation|SetRelativeLocation (Variables|Default|GetCineCamera) (* (Math|Vector|Normalize (Variables|/Script/Engine.SceneComponent|GetRelativeLocation (Variables|Default|GetCineCamera))) NewOrbitDistance) false false))

(fn SetPitchandYawLimits
  (params (NewPitchLimits :type Vector%202D%20Structure) (NewYawLimits :type Vector%202D%20Structure))
  (Variables|CameraAngles|SetMin%20Pitch (.x NewPitchLimits))
  (Variables|CameraAngles|SetMax%20Pitch (.y NewPitchLimits))
  (Variables|CameraAngles|SetMin%20Orbit%20Arc (.x NewYawLimits))
  (Variables|CameraAngles|SetMax%20Orbit%20Arc (.y NewYawLimits))
  (if (< (+ (Variables|CameraAngles|GetMin%20Pitch) (Variables|CameraAngles|GetMax%20Pitch) (Variables|CameraAngles|GetMin%20Orbit%20Arc) (Variables|CameraAngles|GetMax%20Orbit%20Arc)) 0.1)
    (Variables|Default|SetbAllowOrbit false)
    (else
      (Variables|Default|SetbAllowOrbit true))))

(fn ResetPosition
  (Transformation|SetRelativeLocationAndRotation (Variables|Default|GetOrbitPoint) "0, 0, 0" "0, 0, 0" false false)
  (Transformation|SetRelativeLocationAndRotation (Variables|Default|GetPinchOffset) "0, 0, 0" "0, 0, 0" false false)
  (Variables|Default|SetFinalPan 0.0)
  (Variables|Default|SetFinalTrack 0.0)
  (Variables|Default|SetFinalPinch 0.0)
  (Variables|Default|SetPitchAngle 0.0)
  (Variables|Default|SetYawValue 0.0))

(event Custom|Transition
  (params (NewPosition :type Float%20%28double-precision%29) (New%20Pitch :type Float%20%28double-precision%29))
  (Variables|Default|SetTarget%20Yaw NewPosition)
  (Variables|Default|SetbFindTarget true))

(fn StatusUpdate
  (params (Hunger :type Float%20%28double-precision%29))
  (return 0.0))