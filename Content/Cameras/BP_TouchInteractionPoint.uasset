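; Touch hotspot actor that shows a billboard marker in orbit mode and triggers model swaps or power mode on NavigationBP.
; Swiping reveals the marker and restarts a timer that fades it out when idle.
; Tick uses camera distance to set readiness and drive the dynamic material's ring, opacity and color.
; FireEvent alternates the model index when ready, J triggers power mode, and a timeline animates opacity on firing.
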(event Custom|FireEvent
  ;[1 1 1] Interaction routing
  (if (and (Variables|Default|GetbTouchReady) (not (Variables|Default|GetbShouldHide)))
    (Variables|Default|SetbIsFiring true)
    (bind _isa (Utilities|FlowControl|FlipFlop)
      (:A
        _)
      (:B
        _))
    (Default|SwapModel (Variables|Default|GetNavigation%20BP) (Math|Conversions|ToInteger(Boolean) _isa))
    (bind _fadelerp (Timeline|Blue PlayFromStart)
      (:Update
        (Rendering|Material|SetScalarParameterValue (Variables|Default|GetTouchMat) "Opacity" _fadelerp :!class /Script/Engine.MaterialInstanceDynamic))
      (:Finished
        (Variables|Default|SetbIsFiring false)
        (Rendering|SetVisibility (Variables|Default|GetMaterialBillboard) false false)
        (Rendering|Material|SetScalarParameterValue (Variables|Default|GetTouchMat) "Opacity" 1.0 :!class /Script/Engine.MaterialInstanceDynamic)))))

(event Custom|Vis%20Timer
  (bind _touchmat (Variables|Default|GetTouchMat))
  ;[1 1 1] Visibility Timer
  (Variables|Default|SetbShouldHide true)
  (bind _newtrack_0 (Timeline|DisableFade PlayFromStart)
    (:Update
      (Rendering|Material|SetScalarParameterValue _touchmat "Fade" _newtrack_0 :!class /Script/Engine.MaterialInstanceDynamic))
    (:Finished
      (Rendering|SetVisibility (Variables|Default|GetMaterialBillboard) false false)
      (Rendering|Material|SetScalarParameterValue _touchmat "Fade" 1.0 :!class /Script/Engine.MaterialInstanceDynamic))))

(event Custom|SwapModelIndex
  (params (Index :type Integer))
  ;[1 1 1] Interaction routing
  (Variables|Default|SetbIsFiring true)
  (Default|SwapModel (Variables|Default|GetNavigation%20BP) Index)
  (bind _fadelerp (Timeline|Blue PlayFromStart)
    (:Update
      (Rendering|Material|SetScalarParameterValue (Variables|Default|GetTouchMat) "Opacity" _fadelerp :!class /Script/Engine.MaterialInstanceDynamic))
    (:Finished
      (Variables|Default|SetbIsFiring false)
      (Rendering|SetVisibility (Variables|Default|GetMaterialBillboard) false false)
      (Rendering|Material|SetScalarParameterValue (Variables|Default|GetTouchMat) "Opacity" 1.0 :!class /Script/Engine.MaterialInstanceDynamic))))

(event EventTick
  (params (DeltaSeconds :type Float%20%28single-precision%29))
  (bind _returnvalue (Game|GetPlayerCameraManager 0))
  (bind _returnvalue_2 (Transformation|GetActorLocation))
  (bind _interaction_range (Variables|Default|GetInteraction%20Range))
  (bind _touchmat (Variables|Default|GetTouchMat))
  (bind _returnvalue_3 (- _interaction_range 25.0))
  (bind _returnvalue_4 (Camera|GetCameraLocation _returnvalue))
  (bind _returnvalue_5 (- _returnvalue_4 _returnvalue_2))
  (bind _returnvalue_6 (Math|Vector|VectorLength _returnvalue_5))
  ;[1 1 1] Input driving visibility
  (if (not (Variables|Default|GetbIsFiring))
    (if (Variables|Default|GetbIsSwiping)
      (Utilities|Time|SetTimerbyFunctionName 0 "Vis Timer" 3.0 :!label _label)
      (Variables|Default|SetbShouldHide false)
      ;[1 1 1] Make visible if in Orbit mode and near camera
      (Rendering|SetVisibility (Variables|Default|GetMaterialBillboard) (Variables|/Game/Cameras/BP_NavigationMode.BP_NavigationMode_C|GetbInOrbitState (Variables|Default|GetNavigation%20BP)) false)
      (else
        (Utilities|FlowControl|Sequence
          (:then_0
            (Utilities|FlowControl|DoOnce false
              (:Completed
                (goto _label))))
          (:then_1
            _))))
    (Variables|Default|SetbTouchReady (<= _returnvalue_6 _interaction_range))
    (Rendering|Material|SetScalarParameterValue _touchmat "OuterRing" (Math|Float|MapRangeClamped _returnvalue_6 _returnvalue_3 _interaction_range 1.0 0.0) :!class /Script/Engine.MaterialInstanceDynamic)
    (Rendering|Material|SetScalarParameterValue _touchmat "Opacity" (Math|Float|MapRangeClamped _returnvalue_6 (- _returnvalue_3 5e+01) _returnvalue_3 1.0 0.5) :!class /Script/Engine.MaterialInstanceDynamic)
    (Rendering|Material|SetVectorParameterValue (Variables|Default|GetTouchMat) "TouchColor" (Math|Color|Lerp(LinearColor) "(R=1.000000,G=1.000000,B=1.000000,A=1.000000)" "(R=0.081075,G=0.324899,B=0.705000,A=50.000000)" (Math|Float|MapRangeClamped _returnvalue_6 (- _interaction_range 5.0) _interaction_range 1.0 0.0)) :!class /Script/Engine.MaterialInstanceDynamic)))

(event Input|KeyboardEvents|J
  (params (Key :type Key%20Structure :default "None"))
  ;[1 1 1] Interaction routing
  (:Pressed
    (Variables|Default|SetbIsFiring true)
    (Default|PowerMode (Variables|Default|GetNavigation%20BP))
    (bind _fadelerp (Timeline|Blue PlayFromStart)
      (:Update
        (Rendering|Material|SetScalarParameterValue (Variables|Default|GetTouchMat) "Opacity" _fadelerp :!class /Script/Engine.MaterialInstanceDynamic))
      (:Finished
        (Variables|Default|SetbIsFiring false)
        (Rendering|SetVisibility (Variables|Default|GetMaterialBillboard) false false)
        (Rendering|Material|SetScalarParameterValue (Variables|Default|GetTouchMat) "Opacity" 1.0 :!class /Script/Engine.MaterialInstanceDynamic)))))

(fn ConstructionScript
  (bind _returnvalue (Rendering|Material|CreateDynamicMaterialInstance (Variables|Default|GetMaterialBillboard) 0 0 "None" :!class /Script/Engine.PrimitiveComponent))
  (Variables|Default|SetTouchMat _returnvalue))