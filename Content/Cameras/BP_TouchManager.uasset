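; Touch input component for BP_OrbitCamera that turns touch gestures and mouse axes into orbit, pinch, pan and track inputs.
; Touch suspends mouse input until a delay after release, and the Y key toggles it manually.
; Each Tick, single-finger swipe deltas drive orbit, with large jumps rejected.
; Two-finger gestures zero orbit and drive pinch from finger spacing and pan/track from averaged, interpolated touch positions, clamped and remapped through curves.
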(event Custom|EnableMouse
  (Variables|Default|SetbUseMouse true))

(event Custom|PreventMouse
  ;[1 1 1] Manage Touch Input
  (Variables|Default|SetbUseMouse false)
  (Utilities|Time|ClearTimerbyFunctionName 0 "EnableMouse")
  (CallFunction|ClearData)
  (Variables|/Game/Cameras/BP_OrbitCamera.BP_OrbitCamera_C|SetOverallTouch (Variables|Default|GetOrbitBP) true)
  (if (not (|ExclusionZone (stale Input|TouchEvents|InputTouch Location)))
    (|MultiTouchHandling (stale Input|TouchEvents|InputTouch Location) (stale Input|TouchEvents|InputTouch FingerIndex)
      (:then
        _)
      (:else
        _)
      (:moved
        _))
    (Default|CallTouchHappened)))

(event EventBeginPlay
  ;[1 1 1] Manage Mouse Input
)

(event EventTick
  (params (DeltaSeconds :type Float%20%28single-precision%29))
  (bind _orbitbp (Variables|Default|GetOrbitBP))
  (bind _orbitbp_2 (Variables|Default|GetOrbitBP))
  ;[1 1 1] Manage Mouse Input
  (Variables|Default|SetTickTime DeltaSeconds)
  (if (Variables|Default|GetbDisableMouse)
    (Variables|/Game/Cameras/BP_OrbitCamera.BP_OrbitCamera_C|SetMouse%20X _orbitbp 0.0)
    (Variables|/Game/Cameras/BP_OrbitCamera.BP_OrbitCamera_C|SetMouse%20Y _orbitbp 0.0)
    (else
      (Variables|/Game/Cameras/BP_OrbitCamera.BP_OrbitCamera_C|SetMouse%20X _orbitbp_2 (* (Math|Float|SelectFloat (Class|Actor|GetInputAxisKeyValue) 0.0 (stale Input|KeyboardEvents|Y _output_get)) 2.0))
      (Variables|/Game/Cameras/BP_OrbitCamera.BP_OrbitCamera_C|SetMouse%20Y _orbitbp_2 (* (Math|Float|SelectFloat (Class|Actor|GetInputAxisKeyValue) 0.0 (stale Input|KeyboardEvents|Y _output_get)) 2.0))))
  (|SwipeTest)
  (|PinchResults))

(event Input|KeyboardEvents|Y
  (params (Key :type Key%20Structure))
  ;[1 1 1] Manage Mouse Input
  (:Pressed
    (bind _output_get (Variables|Default|SetbUseMouse (not (Variables|Default|GetbUseMouse))))))

(event Input|TouchEvents|Touch1
  (params (Key :type Key%20Structure))
  ;[1 1 1] Manage Touch Input
  (:Pressed
    (Variables|Default|SetTouch1Pressed true)
    (Variables|Default|SetTouchCount (+ (Math|Conversions|ToInteger(Boolean) (Variables|Default|GetTouch1Pressed)) (Math|Conversions|ToInteger(Boolean) (Variables|Default|GetTouch2Pressed))) :!label _label))
  (:Released
    (Variables|Default|SetTouch1Pressed false)
    (goto _label)))

(event Input|TouchEvents|Touch2
  (params (Key :type Key%20Structure))
  ;[1 1 1] Manage Touch Input
  (:Pressed
    (Variables|Default|SetTouch2Pressed true)
    (Variables|Default|SetTouchCount (+ (Math|Conversions|ToInteger(Boolean) (Variables|Default|GetTouch1Pressed)) (Math|Conversions|ToInteger(Boolean) (Variables|Default|GetTouch2Pressed))) :!label _label))
  (:Released
    (Variables|Default|SetTouch2Pressed false)
    (goto _label)))

(event Input|TouchEvents|InputTouch
  (params (Location :type Vector) (FingerIndex :type ETouchIndex%20Enum))
  (bind _result (|ExclusionZone Location))
  (bind _orbitbp (Variables|Default|GetOrbitBP))
  ;[1 1 1] Manage Touch Input
  (:Pressed
    (Variables|Default|SetbUseMouse false)
    (Utilities|Time|ClearTimerbyFunctionName 0 "EnableMouse")
    (CallFunction|ClearData)
    (Variables|/Game/Cameras/BP_OrbitCamera.BP_OrbitCamera_C|SetOverallTouch _orbitbp true)
    (if (not _result)
      (|MultiTouchHandling Location FingerIndex :!label _label
        (:then
          _)
        (:else
          _)
        (:moved
          _))
      (Default|CallTouchHappened)))
  (:Released
    (Variables|/Game/Cameras/BP_OrbitCamera.BP_OrbitCamera_C|SetOverallTouch _orbitbp false)
    (Utilities|Time|SetTimerbyFunctionName 0 "EnableMouse" 1e+01)
    (CallFunction|ClearData))
  (:Moved
    (Variables|/Game/Cameras/BP_OrbitCamera.BP_OrbitCamera_C|SetOverallTouch _orbitbp true)
    (if (not _result)
      (goto _label Move))))

(fn ConstructionScript
  (bind _asbp_orbit_camera (Utilities|Casting|CastToBP_OrbitCamera (Components|GetOwner)))
  (Variables|Default|SetOrbitBP _asbp_orbit_camera))

(event Custom|ClearData
  (Variables|Default|SetTouchTwoLoc "0, 0, 0")
  (Variables|Default|SetTouchOneLoc "0, 0, 0")
  (Variables|Default|SetPrevTouch2Loc "0, 0, 0")
  (Variables|Default|SetPrevTouch1Loc "0, 0, 0")
  (Variables|Default|SetPinchAverage 0.0)
  (Variables|Default|SetInitialPinchLength 0.0)
  (Variables|Default|SetPrevTrack 0.0)
  (Variables|Default|SetPrevPan 0.0))

(event Input|TouchEvents|InputTouch
  (params (Location :type Vector) (FingerIndex :type ETouchIndex%20Enum))
  (:Moved
    (Utilities|FlowControl|Sequence
      (:then_0
        (switch Utilities|FlowControl|Switch|SwitchonETouchIndex FingerIndex
          (:Touch1
            (bind _output_get (Variables|Default|SetNewTouch_A Location)))
          (:Touch2
            (bind _output_get_2 (Variables|Default|SetNewTouch_B Location)))))
      (:then_1
        (Utilities|Array|SetArrayElem (Variables|Default|GetTrackArray) (Variables|Default|GetTrackIndex) (+ _output_get _output_get_2) true)
        (Variables|Default|SetTrackIndex (Math|Integer|SelectInt 0 (+ (Variables|Default|GetTrackIndex) 1) (>= (+ (Variables|Default|GetTrackIndex) 1) 5)))))))