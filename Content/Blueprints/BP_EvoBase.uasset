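; Base AI character for an Evo creature that walks, swims or flies, tracked by the player's orbit camera.
; Runs a behavior tree, seeding its blackboard with abilities and biome laps, and attaches a water ripple component.
; Overlaps, physical-material hits and events switch movement mode, mostly mirrored to the blackboard.
; A looping timer drains hunger to the player's UI, while biome preference calls increment scores shown in a debug widget.
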(event Custom|UpdateHunger
  ;[1 0.6623 0] Updates Hunger Status
  (bind _output_get (Variables|Statuses|SetHunger (Math|Float|Clamp(Float) (- (Variables|Statuses|GetHunger) 0.1))))
  (Class|BIEvoBaseInterface|StatusUpdate(Message) (Variables|/Game/UI/WDP_MainUI.WDP_MainUI_C|GetWDP_Status (Variables|/Game/Blueprints/BP_PlayerPawn.BP_PlayerPawn_C|GetREF_UI_MainUI (stale EventBeginPlay _asbp_player_pawn_2))) _output_get))

(event EventBeginPlay
  (bind _self self)
  (bind _self_2 self)
  (bind _returnvalue (AI|GetAIController _self_2))
  (Utilities|FlowControl|Sequence
    (:then_0
      (bind _returnvalue_2 (Actor|GetActorOfClass "/Game/Blueprints/BP_FlyingVolume.BP_FlyingVolume_C"))
      (if (Collision|IsOverlappingActor _returnvalue_2 :!class /Script/Engine.Actor)
        (Variables|Default|SetREF_EvoMovementMode "NewEnumerator5")
        (Pawn|Components|CharacterMovement|SetMovementMode (Variables|Character|GetCharacterMovement) "MOVE_Flying" 0)))
    (:then_1
      ;[0 0.5 1] Ripples Around Water
      (bind _returnvalue_3 (Game|SpawnActorfromClass "/Water/FluidSimulation/Blueprints/Examples/BP_Dynamic_Force_Component.BP_Dynamic_Force_Component_C" (Transformation|GetWorldTransform (Variables|Character|GetMesh)) "AlwaysSpawn" _self _self))
      (bind _output_get (Variables|Default|SetRippleComponent _returnvalue_3))
      (Transformation|AttachComponentToComponent _returnvalue_3 (Variables|Character|GetMesh) "None" "SnapToTarget" "KeepRelative" "KeepRelative" true)
      (Variables|/Water/FluidSimulation/Blueprints/Examples/BP_Dynamic_Force_Component.BP_Dynamic_Force_Component_C|SetRadius _output_get 5e+01))
    (:then_2
      ;[0 0.5 0.2] Casts to player pawn to get Camera reference
      (bind _asbp_player_pawn (Utilities|Casting|CastToBP_PlayerPawn (Pawn|GetControlledPawn (Game|GetPlayerController 0)))))
    (:then_3
      ;[0 0.5 1] Initializes Behavior Tree
      (AI|RunBehaviorTree _returnvalue (Variables|Default|GetBT_AIBase))
      (AI|Components|Blackboard|SetValueasEnum (Utilities|GetBlackboard) (Utilities|Name|MakeLiteralName "EvoMovementMode") (Variables|Default|GetREF_EvoMovementMode))
      (AI|Components|Blackboard|SetValueasBool (Utilities|GetBlackboard) (Utilities|Name|MakeLiteralName "CanWalk?") (Variables|Movement|GetCanWalk?))
      (AI|Components|Blackboard|SetValueasBool (Utilities|GetBlackboard) (Utilities|Name|MakeLiteralName "CanSwim?") (Variables|Movement|GetCanSwim?))
      (AI|Components|Blackboard|SetValueasBool (Utilities|GetBlackboard) (Utilities|Name|MakeLiteralName "CanFly?") (Variables|Movement|GetCanFly?)))
    (:then_4
      ;[0 0.5 1] Preferred biome
      (Class|BlackboardComponent|SetValueasInt (AI|GetBlackboard _returnvalue) (Utilities|Name|MakeLiteralName "BiomeLaps") (Variables|Default|GetEvoBiomeLaps) :!pinned true) ; Sets Number of laps by default
    )
    (:then_5
      ;[1 0.6623 0] Updates Hunger Status
      (Utilities|Time|SetTimerbyFunctionName 0 "UpdateHunger" 1.0 true)
      (bind _asbp_player_pawn_2 (Utilities|Casting|CastToBP_PlayerPawn (Game|Player|GetPlayerPawn 0))))))

(event EventActorDestroyed
  ;[1 0.6623 0] Updates Hunger Status
  (AI|Components|Blackboard|SetValueasBool (AI|GetBlackboard (AI|GetAIController (Components|GetOwner))) (Utilities|Name|MakeLiteralName "AteFood") true)
  (Variables|Statuses|SetHunger (+ (Variables|Statuses|GetHunger) 5.0)))

(event EventSetFalling
  ;[0 0.5 1] Update Movement Modes
  (CallFunction|UpdateMovementMode "MOVE_Falling"))

(event Collision|EventActorBeginOverlap
  (params (OtherActor :type Actor%20Object%20Reference))
  ;[0 0.5 1] Update Movement Modes
  (Utilities|FlowControl|Sequence
    (:then_0
      (bind _asbp_food_base (Utilities|Casting|CastToBP_FoodBase OtherActor))
      (Development|PrintString (Utilities|String|Append "Overlapping " (Utilities|GetDisplayName _asbp_food_base)) true true "(R=1.000000,G=0.000000,B=0.000000,A=1.000000)")
      (Components|Movement|StopMovementImmediately (Variables|Character|GetCharacterMovement)))
    (:then_1
      (bind _asphysics_volume (Utilities|Casting|CastToPhysicsVolume OtherActor))
      (Variables|Default|SetREF%20Physics%20Volume _asphysics_volume)
      (CallFunction|UpdateMovementMode "MOVE_Swimming"))))

(event EventTick
  (params (DeltaSeconds :type Float%20%28single-precision%29))
  ;[0 0.5 1] Ticks location so camera follows
  (Class|BIEvoBaseInterface|EvoLocation(Message) (Variables|/Game/Blueprints/BP_PlayerPawn.BP_PlayerPawn_C|GetREF_OrbitCamera (stale EventBeginPlay _asbp_player_pawn)) (Transformation|GetActorLocation)))

(event EventSetBiomePreference
  (params (HitBiome :type E_Biomes%20Enum :default "NewEnumerator0") (HitLocation :type Vector :default "0, 0, 0"))
  (bind _output_get (Variables|Default|SetE_Biomes HitBiome))
  (bind _returnvalue (Actor|GetActorOfClass "/Game/Blueprints/BP_PlayerPawn.BP_PlayerPawn_C"))
  (Variables|Default|SetREF_BP_PlayerPawn _returnvalue)
  (switch Utilities|FlowControl|Switch|SwitchonE_Biomes _output_get
    (:NewEnumerator0
      (bind _output_get_2 (Variables|Default|SetBiomeGrassScore (+ (Variables|Default|GetBiomeGrassScore) 1)))
      (Class|BIEvoBaseInterface|SetBiomeScore(Message) (Variables|/Game/UI/WDP_MainUI.WDP_MainUI_C|GetWDP_BiomeScoresDebug (Variables|/Game/Blueprints/BP_PlayerPawn.BP_PlayerPawn_C|GetREF_UI_MainUI (Variables|Default|GetREF_BP_PlayerPawn))) _output_get_2 "NewEnumerator0"))
    (:NewEnumerator1
      (bind _output_get_3 (Variables|Default|SetBiomeCliffScore (+ (Variables|Default|GetBiomeCliffScore) 1)))
      (Class|BIEvoBaseInterface|SetBiomeScore(Message) (Variables|/Game/UI/WDP_MainUI.WDP_MainUI_C|GetWDP_BiomeScoresDebug (Variables|/Game/Blueprints/BP_PlayerPawn.BP_PlayerPawn_C|GetREF_UI_MainUI (Variables|Default|GetREF_BP_PlayerPawn))) _output_get_3 "NewEnumerator1"))
    (:NewEnumerator2
      (bind _output_get_4 (Variables|Default|SetBiomeWaterScore (+ (Variables|Default|GetBiomeWaterScore) 1)))
      (Class|BIEvoBaseInterface|SetBiomeScore(Message) (Variables|/Game/UI/WDP_MainUI.WDP_MainUI_C|GetWDP_BiomeScoresDebug (Variables|/Game/Blueprints/BP_PlayerPawn.BP_PlayerPawn_C|GetREF_UI_MainUI (Variables|Default|GetREF_BP_PlayerPawn))) _output_get_4 "NewEnumerator2"))))

(event Collision|EventHit
  (params (MyComp :type Primitive%20Component%20Object%20Reference) (Other :type Actor%20Object%20Reference) (OtherComp :type Primitive%20Component%20Object%20Reference) (bSelfMoved :type Boolean) (HitLocation :type Vector :default "0, 0, 0") (HitNormal :type Vector :default "0, 0, 0") (NormalImpulse :type Vector :default "0, 0, 0") (Hit :type Hit%20Result%20Structure%20%28by%20ref%29))
  (bind (_bblockinghit _binitialoverlap _time _distance _location _impactpoint _normal _impactnormal _physmat) (Collision|BreakHitResult Hit))
  (bind _charactermovement (Variables|Character|GetCharacterMovement))
  (bind _charactermovement_2 (Variables|Character|GetCharacterMovement))
  (bind _movementmode (Variables|/Script/Engine.CharacterMovementComponent|GetMovementMode _charactermovement))
  (bind _movementmode_2 (Variables|/Script/Engine.CharacterMovementComponent|GetMovementMode _charactermovement_2))
  (if _bblockinghit
    (if (== _physmat "/Game/Materials/PhysMaterials/PM_Grass.PM_Grass")
      (Variables|Default|SetIsInAir? false)
      (Pawn|Components|CharacterMovement|SetMovementMode _charactermovement "MOVE_Walking" 0)
      (AI|Components|Blackboard|SetValueasEnum (Utilities|GetBlackboard) (Utilities|Name|MakeLiteralName "EvoMovementMode") _movementmode)
      (Development|PrintString (Utilities|String|EnumtoString _movementmode))
      (elif (== _physmat "/Game/Materials/PhysMaterials/PM_InWater.PM_InWater")
        (Variables|Default|SetIsInAir? false)
        (Pawn|Components|CharacterMovement|SetMovementMode _charactermovement_2 "MOVE_Swimming" 0)
        (AI|Components|Blackboard|SetValueasEnum (Utilities|GetBlackboard) (Utilities|Name|MakeLiteralName "EvoMovementMode") _movementmode_2)
        (Development|PrintString (Utilities|String|EnumtoString _movementmode_2))))))

(event EventSetFlying
  ;[0 0.5 1] Update Movement Modes
  (Variables|Default|SetIsInAir? true)
  (CallFunction|UpdateMovementMode "MOVE_Flying"))

(fn ConstructionScript)

(fn UpdateMovementMode
  (params (NewMovementMode :type EMovementMode%20Enum :default "MOVE_None"))
  (bind _charactermovement (Variables|Character|GetCharacterMovement))
  (bind _movementmode (Variables|/Script/Engine.CharacterMovementComponent|GetMovementMode _charactermovement))
  (Pawn|Components|CharacterMovement|SetMovementMode _charactermovement NewMovementMode 0)
  (AI|Components|Blackboard|SetValueasEnum (Utilities|GetBlackboard) (Utilities|Name|MakeLiteralName "EvoMovementMode") _movementmode)
  (Development|PrintString (Utilities|String|EnumtoString _movementmode)))

(fn StatusUpdate
  (params (Hunger :type Float%20%28double-precision%29)))