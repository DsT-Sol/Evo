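; BP_FlyingVolume is a volume that sets overlapping EvoBase characters flying.
; On begin overlap it casts the actor to EvoBase and calls SetFlyingMessage if CanFly is true, printing an error if the cast is invalid.
; End overlap does nothing, as the matching SetFallingMessage logic is disconnected and never runs.
; StatusUpdate is a stub that takes Hunger and returns zero.
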(event Collision|EventActorEndOverlap
  (params (OtherActor :type Actor%20Object%20Reference)))

(event Collision|EventActorBeginOverlap
  (params (OtherActor :type Actor%20Object%20Reference))
  (bind _ref_bp_evo_base (CallFunction|CastEvoBase OtherActor))
  (Utilities|IsValid _ref_bp_evo_base
    (:Is%20Valid
      (if (Variables|/Game/Blueprints/BP_EvoBase.BP_EvoBase_C|GetCanFly? _ref_bp_evo_base)
        (Class|BIEvoBaseInterface|SetFlying(Message) _ref_bp_evo_base)))
    (:Is%20Not%20Valid
      (Development|PrintString "Failed to set flying because EvoCharacter is not Valid! Or actor is not EvoBase Class." true true "(R=1.000000,G=0.000000,B=0.000000,A=1.000000)"))))

(event EventBeginPlay)

(fn ConstructionScript)

(fn StatusUpdate
  (params (Hunger :type Float%20%28double-precision%29))
  (return 0.0))