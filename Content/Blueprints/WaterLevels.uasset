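; WaterLevels is an actor with Shallow and MedDeep components, apparently intended to alter BP_EvoBase walking speed in water.
; ShallowWaterWalk flip-flops that character's MaxWalkSpeed between a slow and a faster value, designed to repeat on a looping timer.
; The overlap events are empty: the logic that caches the character and speed, starts the timer, and later restores speed is disconnected.
; The construction script applies BasicShapeMaterial to both components when ShowMesh is set.
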(event Custom|ShallowWaterWalk
  ;[1 1 1] Swimming Movement
  (Utilities|FlowControl|FlipFlop
    (:A
      (Variables|/Script/Engine.CharacterMovementComponent|SetMaxWalkSpeed (Variables|/Script/Engine.Character|GetCharacterMovement (Variables|Default|GetREF%20BP%20Evo%20Base)) 2e+02))
    (:B
      (Variables|/Script/Engine.CharacterMovementComponent|SetMaxWalkSpeed (Variables|/Script/Engine.Character|GetCharacterMovement (Variables|Default|GetREF%20BP%20Evo%20Base)) 6e+02))))

(event Collision|EventActorBeginOverlap
  (params (OtherActor :type Actor%20Object%20Reference))
  ;[1 1 1] Swimming Movement
)

(event Collision|EventActorEndOverlap
  (params (OtherActor :type Actor%20Object%20Reference))
  ;[1 1 1] Swimming Movement
)

(fn ConstructionScript
  (if (Variables|Default|GetShowMesh?)
    (Rendering|Material|SetMaterial (Variables|Default|GetShallow) 0 "/Engine/BasicShapes/BasicShapeMaterial.BasicShapeMaterial")
    (Rendering|Material|SetMaterial (Variables|Default|GetMedDeep) 0 "/Engine/BasicShapes/BasicShapeMaterial.BasicShapeMaterial")))