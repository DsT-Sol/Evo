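; Player pawn for a touch-driven feeding game that picks up food, stacks it in a widget inventory and throws it.
; Toggling the inventory blends from the orbit camera to the nearest feeder camera and spawns food above the inventory widget via screen-to-world deprojection.
; Holding touch builds throw power and aims along a predicted projectile path drawn with spline meshes and an endpoint marker.
; Release throws, then respawns food until the inventory empties.
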(event Custom|SpawnFoodHandler
  ;[1 0.2 0] If enough Food Items in inventory keep spawning until it's empty
  (CallFunction|SpawnFood))

(event Custom|SpawnFood
  ;[0 0.5 0.2] Spawn Food in front of the camera and tags it as "OnScreen"
  (bind _returnvalue (Game|SpawnActorfromClass (stale EventDropItem ItemClass) (CallFunction|GetItemAboveIventoryPosition) "DontSpawnIfColliding" 0 0))
  (bind _asbp_food_base (Utilities|Casting|CastToBP_FoodBase _returnvalue))
  (bind _output_get (Variables|Default|SetREF_FoodBaseChild _asbp_food_base))
  (Physics|SetSimulatePhysics (Variables|/Game/Feeders/BP_FoodBase.BP_FoodBase_C|GetCapsuleCollision _output_get) false)
  (Utilities|Array|Add (Variables|/Script/Engine.Actor|GetTags _output_get) "OnScreen")
  (Audio|PlaySound2D "/Game/Movies/UI_Sounds/UI_ButtonPressed.UI_ButtonPressed" 1.0 1.0 0.0 0 0)
  (Class|BIInventoryInterface|StopLogicandAnim(Message) _output_get))

(event Custom|EnablePhysicsForThrownItems
  ;[0 0.5 0.2] Activate Physics for succesfully thrown objects
  (Physics|SetSimulatePhysics (Variables|/Game/Feeders/BP_FoodBase.BP_FoodBase_C|GetCapsuleCollision (Variables|Default|GetREF_FoodBaseChild)) true)
  (Utilities|FlowControl|Sequence
    (:then_0
      (Utilities|FlowControl|Delay 0.5) ; Time before respawning
      (CallFunction|ReSpawnItemAfterThrown) ; Return Node when empty
      ;[1 0.2 0] Goes back to Orbit Camera when Inventory is empty, and resets main variable during Feeder Cam
      (if (not (Class|PanelWidget|HasAnyChildren (CallFunction|GetInventoryBox)))
        (Utilities|FlowControl|Delay 2.0)
        (Game|Player|SetViewTargetwithBlend (Game|GetPlayerController 0) (Variables|Cameras|GetREF_OrbitCamera) 0.5 "VTBlend_Linear" 0.0 false)
        (Variables|Inventory|SetButtonToggle false)))))

(event Input|EnhancedActionEvents|EnhancedInputActionIA_PickItem
  (params (ActionValue :type Vector%202D%20Structure) (ElapsedSeconds :type Float%20%28double-precision%29) (TriggeredSeconds :type Float%20%28double-precision%29) (InputAction :type Input%20Action%20Object%20Reference :default "/Game/Input/IA_PickItem.IA_PickItem"))
  (bind _returnvalue (Game|GetPlayerController 0))
  (bind _hitresult (Class|PlayerController|GetHitResultUnderFingerbyChannel _returnvalue "Touch1" "TraceTypeQuery1" true))
  (bind _location (Collision|BreakHitResult _hitresult))
  ;[0 0.5 1] Pick up touched items by player
  (:Started
    (bind _outhit (Collision|SphereTraceForObjects _location _location 2e+01 (Utilities|Array|MakeArray "ObjectTypeQuery7") false 0 "Persistent" true "(R=1.000000,G=0.000000,B=0.000000,A=1.000000)" "(R=0.000000,G=0.120050,B=1.000000,A=1.000000)"))
    (bind _asbp_food_base (Utilities|Casting|CastToBP_FoodBase (.HitActor (Collision|BreakHitResult _outhit)))) ; Necesary since food is get by hit
    (bind _output_get (Variables|Default|SetREF_FoodBase _asbp_food_base))
    (if (.bBlockingHit (Collision|BreakHitResult _outhit))
      (if (Variables|Inventory|GetButtonToggle)
        (if (Actor|ActorHasTag _output_get "OnScreen")
          ;[0 0.5 1] Spawn Prediction End Point
          (bind _returnvalue_2 (Game|SpawnActorfromClass "/Game/Blueprints/BP_PredictionEndPoint.BP_PredictionEndPoint_C" (Math|Transform|MakeTransform "0, 0, 0" "0, 0, 0" "1.000000,1.000000,1.000000") "AlwaysSpawn" 0 0))
          (bind _output_get_2 (Variables|PredictionSpline|SetPredictionEndPoint _returnvalue_2))
          (Rendering|SetActorHiddenInGame _output_get_2 false))
        (elif (Actor|ActorHasTag _output_get "Thrown")
          (Development|PrintString "Can't touch this!" true true "(R=1.000000,G=0.000000,B=0.000000,A=1.000000)")
          (else
            (Class|BIInventoryInterface|OnTouchedActor(Message) _output_get self)))))))

(event Input|EnhancedActionEvents|EnhancedInputActionIA_PickItem
  (params (ActionValue :type Vector%202D%20Structure) (ElapsedSeconds :type Float%20%28double-precision%29) (TriggeredSeconds :type Float%20%28double-precision%29) (InputAction :type Input%20Action%20Object%20Reference :default "/Game/Input/IA_PickItem.IA_PickItem"))
  ;[0 0 0 1 20] Throw Food functionality
  (:Triggered
    ;[1 0.2 1] Verifies if in inventory and checks if actor is valid
    (if (Variables|Inventory|GetButtonToggle)
      (bind _ref_foodbase (Variables|Default|GetREF_FoodBase)
        (:then
          (if (Actor|ActorHasTag _ref_foodbase "OnScreen")
            ;[0 0.5 1] Spline Functionality
            (PredictionSpline|CreatePredictionSpline)
            (PredictionSpline|DrawPredictionSpline)
            (PredictionSpline|AddandClampedThrowRotation ActionValue)
            (Utilities|PredictionSplineValid?
              (:Is%20Valid
                (Variables|PredictionSpline|SetStartingTargetPosition (Math|Float|Clamp(Float) (+ (Variables|PredictionSpline|GetStartingTargetPosition) (* TriggeredSeconds (Variables|PredictionSpline|GetTargetMovementVelocity))) 1.4e+03 3e+03))))))
        (:else))))
  (:Completed
    (Utilities|FlowControl|Sequence
      (:then_0
        (PredictionSpline|DestroyPredictionSpline))
      (:then_1
        ;[1 0.2 1] Delete thrown item from stack in inventory
        (bind _ref_foodbase_2 (Variables|Default|GetREF_FoodBase)
          (:then
            (if (Actor|ActorHasTag _ref_foodbase_2 "OnScreen")
              (Default|CallDeleteItemfromStacks)
              (Utilities|Array|Add (Variables|/Script/Engine.Actor|GetTags _ref_foodbase_2) "Thrown")
              (Utilities|Array|RemoveItem (Variables|/Script/Engine.Actor|GetTags _ref_foodbase_2) "OnScreen")
              (Class|BIEvoBaseInterface|SetThrownFoodDirectionandSpeed(Message) _ref_foodbase_2 (Utilities|ThrowVelocity) (Variables|PredictionSpline|GetStartingTargetPosition))
              (Variables|PredictionSpline|SetStartingTargetPosition 1e+03) ; Resets projectile rotation
              (Utilities|Time|SetTimerbyEvent (delegate Custom|EnablePhysicsForThrownItems) 0.1) ; Physics after throwing
            ))
          (:else))))))

(event EventDestroyFoodonToggleChange
  ;[0 0.5 0.2] When Toggle Changes State Food Gets Reeplaced
  (bind _ref_foodbasechild (Variables|Default|GetREF_FoodBaseChild)
    (:then
      (Actor|DestroyActor _ref_foodbasechild))
    (:else)))

(event EventPickUpItem
  (params (ItemClass :type Actor%20Class%20Reference) (ItemIcon :type Texture%202D%20Object%20Reference) (StackAmount :type Integer))
  ;[0 0.5 0.2] Food Items get added to the inventory and stacked
  (CallFunction|AddItemtoInventory ItemClass ItemIcon StackAmount))

(event EventDropItem
  (params (ToggleState :type Boolean) (ItemClass :type Actor%20Class%20Reference))
  ;[1 0.2 0] Camera Switch depending on inventory state
  (bind _output_get (Variables|Inventory|SetButtonToggle ToggleState))
  (if _output_get
    (bind _output_get_2 (Variables|Cameras|SetREF_FeederCamera (CallFunction|GetClosestCameratoOrbitCam)))
    (Game|Player|SetViewTargetwithBlend (Game|GetPlayerController 0) _output_get_2 0.5 "VTBlend_Linear" 0.0 false)
    ;[1 0.2 0] If enough Food Items in inventory keep spawning until it's empty
    (Utilities|Time|SetTimerbyEvent (delegate Custom|SpawnFoodHandler) 0.6)
    (else
      (Game|Player|SetViewTargetwithBlend (Game|GetPlayerController 0) (Variables|Cameras|GetREF_OrbitCamera) 0.5 "VTBlend_Linear" 0.0 false)
      (bind _ref_foodbasechild (Variables|Default|GetREF_FoodBaseChild)
        (:then
          (Actor|DestroyActor _ref_foodbasechild)
          (Variables|Default|SetREF_FoodBaseChild 0))
        (:else)))))

(event EventBeginPlay
  (bind _returnvalue (Game|GetPlayerController 0))
  (bind _returnvalue_2 (PlayerController|LocalPlayerSubsystems|GetEnhancedInputLocalPlayerSubsystem _returnvalue))
  (Utilities|FlowControl|Sequence
    (:then_0
      ;[1 0.2 1] Adds Enhanced Input Mapping
      (Utilities|IsValid _returnvalue_2
        (:Is%20Valid
          (Input|AddMappingContext _returnvalue_2 "/Game/Input/IM_EvoInputMapping.IM_EvoInputMapping" 0 (Utilities|Struct|MakeModifyContextOptions true false)))))
    (:then_1
      ;[1 0.2 0] Sets Orbit Camera as main camera
      (bind _returnvalue_3 (Actor|GetActorOfClass "/Game/Cameras/BP_OrbitCamera.BP_OrbitCamera_C"))
      (Variables|Cameras|SetREF_OrbitCamera _returnvalue_3))
    (:then_2
      ;[0.3 0 1] Adds widget to viewport
      (bind _returnvalue_4 (UserInterface|CreateWidget "/Game/UI/WDP_MainUI.WDP_MainUI_C"))
      (bind _output_get (Variables|Default|SetREF_UI_MainUI _returnvalue_4))
      (UserInterface|Viewport|AddtoViewport _output_get 0))))

(fn ConstructionScript)

(fn AddItemtoInventory
  (params (ItemClass :type Actor%20Class%20Reference) (ItemIcon :type Texture%202D%20Object%20Reference) (MaxStack :type Integer))
  (if (> MaxStack 1)
    (bind _array_element (Utilities|Array|ForEachLoopwithBreak (Class|PanelWidget|GetAllChildren (CallFunction|GetInventoryBox)) :!label _label)
      (:LoopBody
        (bind (_itemclass _currentstackamount _maxstackamount) (Class|BIInventoryInterface|GetPickUpItemData(Message) _array_element))
        (if (== _itemclass ItemClass)
          (if (<= (+ _currentstackamount 1) _maxstackamount)
            (Class|BIInventoryInterface|AddPickUpItemtoStack(Message) _array_element)
            (LocalVariables|SetIsItemAdded? true)
            (goto _label Break))))
      (:Completed
        (if (not (LocalVariables|GetIsItemAdded?))
          (bind _returnvalue (UserInterface|CreateWidget "/Game/UI/WDP_PickUpItems.WDP_PickUpItems_C" :!label _label_2))
          (Variables|/Game/UI/WDP_PickUpItems.WDP_PickUpItems_C|SetItemClass _returnvalue ItemClass)
          (Class|Image|SetBrush (Variables|/Game/UI/WDP_PickUpItems.WDP_PickUpItems_C|GetItemIcon _returnvalue) (Class|WidgetBlueprintLibrary|MakeBrushfromTexture ItemIcon 85 85))
          (Variables|/Game/UI/WDP_PickUpItems.WDP_PickUpItems_C|SetMaxStack _returnvalue MaxStack)
          (Class|WrapBox|AddChildtoWrapBox (CallFunction|GetInventoryBox) _returnvalue))))
    (else
      (goto _label_2))))

(fn CreatePredictionSpline
  (bind _returnvalue (AddComponent|AddSplineComponent false))
  (Variables|PredictionSpline|SetPredictionSpline _returnvalue))

(fn DestroyPredictionSpline
  (bind _predictionspline (Variables|PredictionSpline|GetPredictionSpline)
    (:then
      (Components|DestroyComponent _predictionspline)
      (Variables|PredictionSpline|SetPredictionSpline 0)
      (PredictionSpline|DestroyPredictionMeshes)
      (Actor|DestroyActor (Variables|PredictionSpline|GetPredictionEndPoint))
      (Variables|PredictionSpline|SetPredictionEndPoint 0))
    (:else)))

(fn DestroyPredictionMeshes
  (bind _splinemeshes (Variables|PredictionSpline|GetSplineMeshes))
  (for _array_element _splinemeshes
    (Components|DestroyComponent _array_element))
  (Utilities|Array|Clear _splinemeshes))

(fn DrawPredictionSpline
  (bind _predictionendpoint (Variables|PredictionSpline|GetPredictionEndPoint))
  (Utilities|PredictionSplineValid?
    (:Is%20Valid
      (Utilities|FlowControl|Sequence
        (:then_0
          (bind (_outhit _outpathpositions _outlasttracedestination _returnvalue) (Class|GameplayStatics|BlueprintPredictProjectilePathbyTraceChannel (Utilities|ThrowLocation) (Utilities|ThrowVelocity) true 2e+01 "ECC_WorldDynamic" false (Utilities|Array|MakeArray self (Variables|Default|GetREF_FoodBase)) "None" 0.0 15.0 3.0))
          (if _returnvalue
            (Rendering|SetActorHiddenInGame _predictionendpoint false)
            (Transformation|SetActorLocation (Variables|PredictionSpline|GetPredictionEndPoint) (.ImpactPoint (Collision|BreakHitResult _outhit)) false true)
            (else
              (Rendering|SetActorHiddenInGame _predictionendpoint true)))
          (Spline|SetSplinePoints (Variables|PredictionSpline|GetPredictionSpline) _outpathpositions "World" true)
          (PredictionSpline|DestroyPredictionMeshes))
        (:then_1
          ;[1 1 1] Spline Construction
          (for _index (range 0 (Math|Float|Truncate (/ (Spline|GetSplineLength (Variables|PredictionSpline|GetPredictionSpline)) 1e+02)))
            (LocalVariables|SetIndex _index)
            (bind _returnvalue_2 (AddComponent|AddSplineMeshComponent true))
            (Utilities|Array|Add (Variables|PredictionSpline|GetSplineMeshes) _returnvalue_2)
            (SplineMesh|SetStartandEnd _returnvalue_2 (Spline|GetLocationatDistanceAlongSpline (Variables|PredictionSpline|GetPredictionSpline) (* (LocalVariables|GetIndex) 1e+02) "World") (Math|Vector|ClampVectorSize (Spline|GetTangentatDistanceAlongSpline (Variables|PredictionSpline|GetPredictionSpline) (* (LocalVariables|GetIndex) 1e+02) "World") 0.0 1e+02) (Spline|GetLocationatDistanceAlongSpline (Variables|PredictionSpline|GetPredictionSpline) (* (+ (LocalVariables|GetIndex) 1) 1e+02) "World") (Math|Vector|ClampVectorSize (Spline|GetTangentatDistanceAlongSpline (Variables|PredictionSpline|GetPredictionSpline) (* (+ (LocalVariables|GetIndex) 1) 1e+02) "World") 0.0 1e+02) true :!class /Script/Engine.SplineMeshComponent)))))))

(fn AddandClampedThrowRotation
  (params (RotationAxis :type Vector%202D%20Structure))
  (bind _ref_feedercamera (Variables|Cameras|GetREF_FeederCamera))
  (bind _throwtransform (Variables|/Game/Cameras/BP_FeederCamera.BP_FeederCamera_C|GetThrowTransform _ref_feedercamera))
  (bind _relativerotation (Variables|/Script/Engine.SceneComponent|GetRelativeRotation _throwtransform))
  (Transformation|SetRelativeRotation _throwtransform (Math|Rotator|MakeRotator (.roll _relativerotation) (.pitch _relativerotation) (Math|Float|Clamp(Float) (+ (/ (- (.X (Math|Vector2D|BreakVector2D RotationAxis)) (/ (.x (Viewport|GetViewportSize)) 2.0)) 1e+03) (.yaw _relativerotation)) -5e+01 5e+01)) false false))

(fn ResetFeederCamRotation
  (Transformation|SetRelativeRotation (Variables|/Game/Cameras/BP_FeederCamera.BP_FeederCamera_C|GetThrowTransform (Variables|Cameras|GetREF_FeederCamera)) "30.000000,0.000000,0.000000" false false))

(fn ReSpawnItemAfterThrown
  ;[1 1 1] Items keep spawning when selected
  (if (> (Class|PanelWidget|GetChildrenCount (CallFunction|GetInventoryBox)) 0)
    (CallFunction|SpawnFood)
    (else
      (return))))

(fn GetInventoryBox
  (return (Variables|/Game/UI/WDP_Inventory.WDP_Inventory_C|GetInventoryBox (Variables|/Game/UI/WDP_MainUI.WDP_MainUI_C|GetWDP_Inventory (Variables|Default|GetREF_UI_MainUI)))))

(fn GetItemAboveIventoryPosition
  (bind _returnvalue (Game|GetPlayerController 0))
  (bind _ref_ui_mainui (Variables|Default|GetREF_UI_MainUI))
  (bind _wdp_inventory (Variables|/Game/UI/WDP_MainUI.WDP_MainUI_C|GetWDP_Inventory _ref_ui_mainui))
  (bind _returnvalue_2 (Class|Widget|GetCachedGeometry _wdp_inventory))
  (bind _pixelposition (Class|SlateBlueprintLibrary|LocaltoViewport _returnvalue_2))
  (bind _returnvalue_3 (Class|SlateBlueprintLibrary|GetAbsoluteSize _returnvalue_2))
  (bind (_x _y) (Math|Vector2D|BreakVector2D _pixelposition))
  (bind _returnvalue_4 (/ (.x _returnvalue_3) 2.0))
  (bind _returnvalue_5 (* (.y _returnvalue_3) 2.0))
  (bind _returnvalue_6 (+ _x _returnvalue_4))
  (bind _returnvalue_7 (- _y _returnvalue_5))
  (bind (_worldposition _worlddirection) (Class|GameplayStatics|DeprojectScreentoWorld _returnvalue (Math|Vector2D|MakeVector2D _returnvalue_6 _returnvalue_7)))
  (return (Math|Transform|MakeTransform (+ _worldposition (* _worlddirection (Variables|PredictionSpline|GetFoodItemForwardPosition))))))

(fn GetClosestCameratoOrbitCam
  (bind _cameradistancemap (LocalVariables|GetCameraDistanceMap))
  (bind _outactors (Actor|GetAllActorsOfClass "/Game/Cameras/BP_FeederCamera.BP_FeederCamera_C"))
  (bind _output_get (LocalVariables|SetFeederCamsArray _outactors))
  (for _array_element _output_get
    (Utilities|Map|Add _cameradistancemap _array_element (Math|Vector|VectorLength (- (Transformation|GetWorldLocation (Variables|/Game/Cameras/BP_FeederCamera.BP_FeederCamera_C|GetCamera _array_element)) (Transformation|GetWorldLocation (Variables|/Game/Cameras/BP_OrbitCamera.BP_OrbitCamera_C|GetCineCamera (Variables|Cameras|GetREF_OrbitCamera))))))
    (bind _values (Utilities|Map|Values _cameradistancemap))
    (bind _keys (Utilities|Map|Keys _cameradistancemap)))
  (bind _output_get_2 (LocalVariables|SetClosestFeederCam (Utilities|Array|Get(acopy) _keys (.IndexOfMinValue (Math|Float|MinOfFloatArray _values)))))
  (Utilities|Map|Clear (LocalVariables|GetCameraDistanceMap))
  (return _output_get_2))

(fn GetPickUpItemData
  (return 0 0 0))

(fn StatusUpdate
  (params (Hunger :type Float%20%28double-precision%29))
  (return Hunger))