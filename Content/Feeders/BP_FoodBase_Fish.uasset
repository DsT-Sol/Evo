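; BP_FoodBase_Fish is an AI-driven fish food actor that runs a fish behavior tree and caches the level's fish patrol path.
; A per-frame looping timer drives forward movement input, pausing once the fish nears its move target.
; Stopping logic unpossesses it, halts animation, resizes the capsule and reorients the mesh relative to the camera.
; Vanish events wait on a timer, then fade a dynamic material via timeline before destroying the actor.
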(event Custom|VanishTimer
  (bind _returnvalue (Rendering|Material|CreateDynamicMaterialInstance (Variables|Default|GetSkeletalMesh) 0 "/Game/Materials/MI_Vanish.MI_Vanish" "None" :!class /Script/Engine.PrimitiveComponent))
  (bind _vanishtrack (Timeline|Timeline_0 Play)
    (:Update
      (Rendering|Material|SetScalarParameterValue _returnvalue "Vanish" _vanishtrack :!class /Script/Engine.MaterialInstanceDynamic))
    (:Finished
      (Actor|DestroyActor))))

(event Custom|GetThere
  (bind _self self)
  ;[1 1 1] Add Movement From AI
  (Pawn|Input|AddMovementInput _self (Transformation|GetActorForwardVector _self) 1.0 false)
  (if (Utilities|Operators|EqualEqual (Transformation|GetActorLocation self) (stale EventEventAddMovement MoveTarget) 1e+02)
    (Utilities|Time|PauseTimerbyHandle (stale EventEventAddMovement _returnvalue))))

(event EventBeginPlay
  (|CallParentFunction)
  (AI|RunBehaviorTree (AI|GetAIController self) (Variables|Default|GetREF_BTTFish))
  (bind _returnvalue (Actor|GetActorOfClass "/Game/AI/BP_FishPatrolPath.BP_FishPatrolPath_C"))
  (Variables|Default|SetREF_FeederPatrolPath _returnvalue))

(event Collision|EventActorBeginOverlap
  (params (OtherActor :type Actor%20Object%20Reference))
  (|CallParentFunction OtherActor) ; This node is disabled and will not be called.\nDrag off pins to build functionality.
)

(event EventTick
  (params (DeltaSeconds :type Float%20%28single-precision%29)))

(event EventStopLogicandAnim
  (bind _returnvalue (Game|GetPlayerCameraManager 0))
  (bind _capsulecollision (Variables|Default|GetCapsuleCollision))
  (bind _returnvalue_2 (Camera|GetCameraRotation _returnvalue))
  (bind (_roll _pitch _yaw) (Math|Rotator|BreakRotator _returnvalue_2))
  (Pawn|UnPossess (AI|GetAIController self))
  (Audio|Components|Audio|Stop (Variables|Default|GetSkeletalMesh))
  (Components|Capsule|SetCapsuleHalfHeight _capsulecollision 8e+01 true)
  (Components|Capsule|SetCapsuleRadius _capsulecollision 8e+01 true)
  (Transformation|SetRelativeTransform (Variables|Default|GetSkeletalMesh) (Math|Transform|MakeTransform "-20.000000,-20.000000,0.000000" "0, 0, 0" "0.500000,2.000000,0.500000") false false)
  (Transformation|SetRelativeRotation (Variables|Default|GetSkeletalMesh) (Math|Rotator|MakeRotator (+ _roll -1e+01) (- _pitch -2e+01) (+ _yaw 9e+01)) false false))

(event EventVanishItemonWater
  (Utilities|Time|SetTimerbyEvent (delegate Custom|VanishTimer) (Variables|Default|GetTimeBeforeVanish)))

(event EventVanishItem
  (Utilities|Time|SetTimerbyEvent (delegate Custom|VanishTimer) (Variables|Default|GetTimeBeforeVanish)))

(event EventEventAddMovement
  (params (MoveTarget :type Vector :default "0, 0, 0"))
  ;[1 1 1] Add Movement From AI
  (bind _returnvalue (Utilities|Time|SetTimerbyEvent (delegate Custom|GetThere) (Utilities|Time|GetWorldDeltaSeconds) true)))

(fn ConstructionScript
  (|CallParentFunction))