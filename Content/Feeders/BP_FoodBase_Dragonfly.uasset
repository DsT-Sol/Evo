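; Dragonfly food actor that runs a behavior tree through its AI controller on BeginPlay.
; StopLogicandAnim unpossesses the controller, stops the skeletal animation, resets the mesh offset and resizes the capsule.
; VanishItem and VanishItemonWater share a delay timer, after which every mesh material becomes a dynamic vanish instance.
; A timeline drives their Vanish parameter, then destroys the actor.
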(event Custom|VanishTimer
  (bind _skeletalmesh (Variables|Default|GetSkeletalMesh))
  (for _index (range 0 (Rendering|Material|GetNumMaterials _skeletalmesh))
    (bind _returnvalue (Rendering|Material|CreateDynamicMaterialInstance _skeletalmesh _index "/Game/Materials/MI_Vanish.MI_Vanish" "None" :!class /Script/Engine.PrimitiveComponent))
    (Utilities|Array|Add (Variables|Default|GetDMI_Dragonfly) _returnvalue))
  (bind _vanishtrack (Timeline|Timeline Play)
    (:Update
      (for _array_element (Variables|Default|GetDMI_Dragonfly)
        (Rendering|Material|SetScalarParameterValue _array_element "Vanish" _vanishtrack :!class /Script/Engine.MaterialInstanceDynamic)))
    (:Finished
      (Actor|DestroyActor))))

(event EventBeginPlay
  (|CallParentFunction)
  (AI|RunBehaviorTree (AI|GetAIController self) "/Game/Feeders/DragonflyAI/BTT_Dragonfly.BTT_Dragonfly"))

(event Collision|EventActorBeginOverlap
  (params (OtherActor :type Actor%20Object%20Reference))
  (|CallParentFunction OtherActor) ; This node is disabled and will not be called.\nDrag off pins to build functionality.
)

(event EventTick
  (params (DeltaSeconds :type Float%20%28single-precision%29))
  (|CallParentFunction DeltaSeconds) ; This node is disabled and will not be called.\nDrag off pins to build functionality.
)

(event EventStopLogicandAnim
  (bind _capsulecollision (Variables|Default|GetCapsuleCollision))
  (Pawn|UnPossess (AI|GetAIController self))
  (Audio|Components|Audio|Stop (Variables|Default|GetSkeletalMesh))
  (Transformation|SetRelativeLocation (Variables|Default|GetSkeletalMesh) "0, 0, 0" false false)
  (Components|Capsule|SetCapsuleHalfHeight _capsulecollision 45.0 true)
  (Components|Capsule|SetCapsuleRadius _capsulecollision 45.0 true))

(event EventVanishItemonWater
  (Utilities|Time|SetTimerbyEvent (delegate Custom|VanishTimer) (Variables|Default|GetTimeBeforeVanish)))

(event EventVanishItem
  (Utilities|Time|SetTimerbyEvent (delegate Custom|VanishTimer) (Variables|Default|GetTimeBeforeVanish)))

(fn ConstructionScript
  (|CallParentFunction))