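; BP_FoodBase is the base food item that can be picked up into inventory, thrown, or eaten when overlapped by BP_EvoBase.
; Throws drive the ProjectileMovement velocity and speed.
; A thrown item's first blocking hit sends Evo a biome preference from grass or cliff physical materials, while water entry through Buoyancy sends another.
; Both landings call vanish events, left empty here alongside movement and data stubs.
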(event OnComponentHit(CapsuleCollision)
  (params (HitComponent :type Primitive%20Component%20Object%20Reference) (OtherActor :type Actor%20Object%20Reference) (OtherComp :type Primitive%20Component%20Object%20Reference) (NormalImpulse :type Vector :default "0, 0, 0") (Hit :type Hit%20Result%20Structure%20%28by%20ref%29))
  (bind (_bblockinghit _binitialoverlap _time _distance _location _impactpoint _normal _impactnormal _physmat) (Collision|BreakHitResult Hit))
  (if (Math|Boolean|ANDBoolean (== (Variables|Default|GetNumberOfHits) 0) (Actor|ActorHasTag "Thrown") _bblockinghit)
    (CallFunction|VanishItem)
    (Variables|Default|SetNumberOfHits 1)
    (if (== _physmat "/Game/Materials/PhysMaterials/PM_Grass.PM_Grass")
      (Variables|Default|SetE_Biomes "NewEnumerator0")
      (Class|BIEvoBaseInterface|SetBiomePreference(Message) (Variables|Default|GetREF_BP_EvoBase) (Variables|Default|GetE_Biomes) "0, 0, 0" :!label _label)
      (elif (== _physmat "/Game/Materials/PhysMaterials/PM_Cliff.PM_Cliff")
        (Variables|Default|SetE_Biomes "NewEnumerator1")
        (goto _label)))))

(event OnEnteredWaterDelegate(Buoyancy)
  (params (Pontoon :type Spherical%20Pontoon%20Structure%20%28by%20ref%29))
  (bind _returnvalue (Actor|ActorHasTag "Thrown"))
  (Utilities|FlowControl|Sequence
    (:then_0
      (if _returnvalue
        (Class|BIEvoBaseInterface|SetBiomePreference(Message) (Variables|Default|GetREF_BP_EvoBase) "NewEnumerator2" "0, 0, 0")))
    (:then_1
      (if _returnvalue
        (CallFunction|VanishItemonWater)))))

(event Custom|EventAddMovement
  (params (MoveTarget :type Vector)))

(event Custom|VanishItem)

(event Custom|VanishItemOnWater)

(event EventBeginPlay
  (Physics|SetEnableGravity (Variables|Default|GetCapsuleCollision) (Variables|Default|GetGravity))
  (Variables|Default|SetREF_BP_EvoBase (CallFunction|GetEvoBase)))

(event Collision|EventActorBeginOverlap
  (params (OtherActor :type Actor%20Object%20Reference))
  ;[0 0.5 1] When overlapped by Evo, food gets eaten
  (bind _asbp_evo_base (Utilities|Casting|CastToBP_EvoBase OtherActor))
  (bind _output_get (Variables|Default|SetREF_BP_EvoBase _asbp_evo_base))
  (Actor|DestroyActor)
  (Class|BIEvoBaseInterface|ActorDestroyed(Message) _output_get))

(event EventOnTouchedActor
  (params (TriggerActor :type Actor%20Object%20Reference))
  ;[0.3 0 1] Touched actor goes into inventory
  (Utilities|IsValid TriggerActor
    (:Is%20Valid
      (Class|BIInventoryInterface|PickUpItem(Message) TriggerActor (Variables|Default|GetItemClass) (Variables|Default|GetItemIcon) (Variables|Default|GetStackSize))
      (Actor|DestroyActor))))

(event Collision|EventHit
  (params (MyComp :type Primitive%20Component%20Object%20Reference) (Other :type Actor%20Object%20Reference) (OtherComp :type Primitive%20Component%20Object%20Reference) (bSelfMoved :type Boolean) (HitLocation :type Vector :default "0, 0, 0") (HitNormal :type Vector :default "0, 0, 0") (NormalImpulse :type Vector :default "0, 0, 0") (Hit :type Hit%20Result%20Structure%20%28by%20ref%29))
  ;[0 0.5 1] Item gets hit by other actors
  (Physics|AddForce (Variables|Default|GetCapsuleCollision) (* (Math|Vector|Normalize HitNormal) -1.0) "None" false))

(event EventSetThrownFoodDirectionandSpeed
  (params (ThrowVelocity :type Vector :default "0, 0, 0") (ThrowSpeed :type Float%20%28double-precision%29))
  (bind _projectilemovement (Variables|Default|GetProjectileMovement))
  ;[0 0.5 1] Throws item into world
  (Variables|/Script/Engine.MovementComponent|SetVelocity _projectilemovement ThrowVelocity)
  (Variables|/Script/Engine.ProjectileMovementComponent|SetInitialSpeed _projectilemovement ThrowSpeed)
  (Variables|/Script/Engine.ProjectileMovementComponent|SetMaxSpeed _projectilemovement ThrowSpeed)
  (Variables|/Script/Engine.ProjectileMovementComponent|SetProjectileGravityScale _projectilemovement 1.0))

(fn ConstructionScript)

(fn GetPickUpItemData
  (return 0 0 0))

(fn StatusUpdate
  (params (Hunger :type Float%20%28double-precision%29))
  (return 0.0))