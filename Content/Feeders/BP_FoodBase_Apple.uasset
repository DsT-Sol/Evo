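; BP_FoodBase_Apple is a food actor, named as an apple, that dissolves and removes itself after a delay.
; VanishItem and VanishItemonWater both start a one-shot timer lasting TimeBeforeVanish.
; When it fires, a dynamic MI_Vanish material is applied to the static mesh and a timeline drives its Vanish parameter, destroying the actor when finished.
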(event Custom|VanishTimer
  (bind _returnvalue (Rendering|Material|CreateDynamicMaterialInstance (Variables|Default|GetStaticMesh) 0 "/Game/Materials/MI_Vanish.MI_Vanish" "None" :!class /Script/Engine.PrimitiveComponent))
  (bind _vanishtrack (Timeline|Timeline Play)
    (:Update
      (Rendering|Material|SetScalarParameterValue _returnvalue "Vanish" _vanishtrack :!class /Script/Engine.MaterialInstanceDynamic))
    (:Finished
      (Actor|DestroyActor))))

(event EventBeginPlay
  (|CallParentFunction) ; This node is disabled and will not be called.\nDrag off pins to build functionality.
)

(event Collision|EventActorBeginOverlap
  (params (OtherActor :type Actor%20Object%20Reference))
  (|CallParentFunction OtherActor) ; This node is disabled and will not be called.\nDrag off pins to build functionality.
)

(event EventTick
  (params (DeltaSeconds :type Float%20%28single-precision%29))
  (|CallParentFunction DeltaSeconds) ; This node is disabled and will not be called.\nDrag off pins to build functionality.
)

(event EventVanishItem
  (Utilities|Time|SetTimerbyEvent (delegate Custom|VanishTimer) (Variables|Default|GetTimeBeforeVanish)))

(event EventVanishItemonWater
  (Utilities|Time|SetTimerbyEvent (delegate Custom|VanishTimer) (Variables|Default|GetTimeBeforeVanish)))

(fn ConstructionScript
  (|CallParentFunction))